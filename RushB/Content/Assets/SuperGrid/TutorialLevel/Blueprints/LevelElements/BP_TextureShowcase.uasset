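; BP_TextureShowcase is a tutorial-level display actor that presents the channels of one SuperGrid texture set under a title.
; The construction script sets the title text from TitleString, then switches on TextureSet to assign per-channel utility materials (R, G, B, roughness) for Basic, Dot, Stone or Modern Grid.
; The Basic Grid branch leaves its fourth material input empty.
; All setup happens at construction, with no runtime logic.
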(event EventBeginPlay)

(event Collision|EventActorBeginOverlap
  (params (OtherActor :type Actor%20Object%20Reference)))

(event EventTick
  (params (DeltaSeconds :type Float%20%28single-precision%29)))

(fn ConstructionScript
  (Rendering|Components|TextRender|SetText (Variables|Default|GetTitle) (Utilities|Text|ToText(String) (Variables|Settings|GetTitleString)))
  (switch int (Variables|Settings|GetTextureSet)
    (:1
      ;[1 1 1] Assign BasicGrid textures
      (Rendering|Material|SetMaterial 0 "/Game/Assets/SuperGrid/TutorialLevel/Utility/MaterialInstances/M_Utility_Channel_R.M_Utility_Channel_R")
      (Rendering|Material|SetMaterial 0 "/Game/Assets/SuperGrid/TutorialLevel/Utility/MaterialInstances/M_Utility_Channel_G.M_Utility_Channel_G")
      (Rendering|Material|SetMaterial 0 "/Game/Assets/SuperGrid/TutorialLevel/Utility/MaterialInstances/M_Utility_Channel_B.M_Utility_Channel_B")
      (Rendering|Material|SetMaterial 0 0))
    (:2
      ;[1 1 1] Assign DotGrid textures
      (Rendering|Material|SetMaterial 0 "/Game/Assets/SuperGrid/TutorialLevel/Utility/MaterialInstances/M_Utility_Channel_R_2.M_Utility_Channel_R_2")
      (Rendering|Material|SetMaterial 0 "/Game/Assets/SuperGrid/TutorialLevel/Utility/MaterialInstances/M_Utility_Channel_G_2.M_Utility_Channel_G_2")
      (Rendering|Material|SetMaterial 0 "/Game/Assets/SuperGrid/TutorialLevel/Utility/MaterialInstances/M_Utility_Channel_B_2.M_Utility_Channel_B_2")
      (Rendering|Material|SetMaterial 0 "/Game/Assets/SuperGrid/TutorialLevel/Utility/MaterialInstances/M_Utility_Channel_Rough_2.M_Utility_Channel_Rough_2"))
    (:3
      ;[1 1 1] Assign Stone Grid textures
      (Rendering|Material|SetMaterial 0 "/Game/Assets/SuperGrid/TutorialLevel/Utility/MaterialInstances/M_Utility_Channel_R_3.M_Utility_Channel_R_3")
      (Rendering|Material|SetMaterial 0 "/Game/Assets/SuperGrid/TutorialLevel/Utility/MaterialInstances/M_Utility_Channel_G_3.M_Utility_Channel_G_3")
      (Rendering|Material|SetMaterial 0 "/Game/Assets/SuperGrid/TutorialLevel/Utility/MaterialInstances/M_Utility_Channel_B_3.M_Utility_Channel_B_3")
      (Rendering|Material|SetMaterial 0 "/Game/Assets/SuperGrid/TutorialLevel/Utility/MaterialInstances/M_Utility_Channel_Rough_3.M_Utility_Channel_Rough_3"))
    (:4
      ;[1 1 1] Assign Modern Grid textures
      (Rendering|Material|SetMaterial 0 "/Game/Assets/SuperGrid/TutorialLevel/Utility/MaterialInstances/M_Utility_Channel_R_4.M_Utility_Channel_R_4")
      (Rendering|Material|SetMaterial 0 "/Game/Assets/SuperGrid/TutorialLevel/Utility/MaterialInstances/M_Utility_Channel_G_4.M_Utility_Channel_G_4")
      (Rendering|Material|SetMaterial 0 "/Game/Assets/SuperGrid/TutorialLevel/Utility/MaterialInstances/M_Utility_Channel_B_4.M_Utility_Channel_B_4")
      (Rendering|Material|SetMaterial 0 "/Game/Assets/SuperGrid/TutorialLevel/Utility/MaterialInstances/M_Utility_Channel_Rough_4.M_Utility_Channel_Rough_4"))))